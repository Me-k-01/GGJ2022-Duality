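; Great spider enemy Blueprint that patrols between four MovePoint targets, starting at BeginPlay.
; A custom Walk event chains AI MoveTo calls through the points in order, pausing a random few seconds after each and restarting after the last.
; Failed moves continue like successful ones, but an invalid point among the first three, checked after its move and pause, halts the loop.
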(event `self.ReceiveBeginPlay`
  ;[1 1 1] Run Walk
  (`self.Walk`))

(event `Walk`
  (`|AIMoveTo` self (0.0 0.0 0.0) (`self.MovePoint1`)
    (:`OnSuccess`
      _)
    (:`OnFail`
      _))
  (`KismetSystemLibrary.Delay` (`KismetMathLibrary.RandomFloatInRange` (`KismetMathLibrary.Abs` 1.0) (`KismetMathLibrary.Abs` 10.0)))
  (`/Engine/EditorBlueprintResources/StandardMacros.IsValid` (`self.MovePoint1`)
    (:`Is Valid`
      (`|AIMoveTo` self (0.0 0.0 0.0) (`self.MovePoint2`)
        (:`OnSuccess`
          _)
        (:`OnFail`
          _))
      (`KismetSystemLibrary.Delay` (`KismetMathLibrary.RandomFloatInRange` (`KismetMathLibrary.Abs` 1.0) (`KismetMathLibrary.Abs` 10.0)))
      (`/Engine/EditorBlueprintResources/StandardMacros.IsValid` (`self.MovePoint2`)
        (:`Is Valid`
          (`|AIMoveTo` self (0.0 0.0 0.0) (`self.MovePoint3`)
            (:`OnSuccess`
              _)
            (:`OnFail`
              _))
          (`KismetSystemLibrary.Delay` (`KismetMathLibrary.RandomFloatInRange` (`KismetMathLibrary.Abs` 1.0) (`KismetMathLibrary.Abs` 10.0)))
          (`/Engine/EditorBlueprintResources/StandardMacros.IsValid` (`self.MovePoint3`)
            (:`Is Valid`
              (`|AIMoveTo` self (0.0 0.0 0.0) (`self.MovePoint4`)
                (:`OnSuccess`
                  _)
                (:`OnFail`
                  _))
              (`KismetSystemLibrary.Delay` (`KismetMathLibrary.RandomFloatInRange` (`KismetMathLibrary.Abs` 1.0) (`KismetMathLibrary.Abs` 10.0)))
              (`self.Walk`))))))))

(fn `UserConstructionScript`)